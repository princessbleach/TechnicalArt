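; BP_GlowOrb is a material demo actor whose glowing orb changes appearance at runtime in response to number keys.
; On BeginPlay it enables player input and applies a dynamic instance of M_DemoGlow to the Orb component.
; Keys 1, 2 and 3 set that instance's base colour, glow strength and opacity parameters respectively, with key 1 also printing a debug message.
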(event EventBeginPlay
  (Input|EnableInput (Game|GetPlayerController 0))
  (bind _returnvalue (Rendering|Material|CreateDynamicMaterialInstance (Variables|Default|GetOrb) 0 "/Game/Materials/M_DemoGlow.M_DemoGlow" "None" :!class /Script/Engine.PrimitiveComponent))
  (bind _output_get (Variables|Default|SetDMI_Orb _returnvalue))
  (Rendering|Material|SetMaterial (Variables|Default|GetOrb) 0 _output_get))

(event Collision|EventActorBeginOverlap
  (params (OtherActor :type Actor%20Object%20Reference)))

(event EventTick
  (params (DeltaSeconds :type Float%20%28single-precision%29)))

(event Input|KeyboardEvents|1
  (params (Key :type Key%20Structure :default "None"))
  (:Pressed
    (Rendering|Material|SetVectorParameterValue (Variables|Default|GetDMI_Orb) "BaseColour" "(R=0.463908,G=1.000000,B=0.944986,A=1.000000)" :!class /Script/Engine.MaterialInstanceDynamic)
    (Development|PrintString "Hello")))

(event Input|KeyboardEvents|2
  (params (Key :type Key%20Structure :default "None"))
  (:Pressed
    (Rendering|Material|SetScalarParameterValue (Variables|Default|GetDMI_Orb) "GlowStrength" 2e+01 :!class /Script/Engine.MaterialInstanceDynamic)))

(event Input|KeyboardEvents|3
  (params (Key :type Key%20Structure :default "None"))
  (:Pressed
    (Rendering|Material|SetScalarParameterValue (Variables|Default|GetDMI_Orb) "OpacityLevel" 1e+02 :!class /Script/Engine.MaterialInstanceDynamic)))

(fn ConstructionScript)