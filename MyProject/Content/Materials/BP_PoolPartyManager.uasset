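; BP_PoolPartyManager is a manager actor that animates the day-cycle lighting and material look of a pool party scene.
; On BeginPlay, the TL_DayCycle timeline plays and writes neon level and colour, caustics intensity and sun intensity into the MPC_PoolParty material parameter collection.
; The same timeline drives the SunLight's intensity and tints it with the sky colour track, keeping materials and lighting in sync.
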(event EventBeginPlay
  (bind _sunlight (Variables|Default|GetSunLight))
  (bind (_direction _neonlevel _causticsintensity _sunintensity _skytint _neontint) (Timeline|TL_DayCycle Play)
    (:Update
      (Rendering|Material|SetScalarParameterValue "/Game/Materials/MPC_PoolParty.MPC_PoolParty" "NeonLevel" _neonlevel :!class /Script/Engine.KismetMaterialLibrary)
      (Rendering|Material|SetScalarParameterValue "/Game/Materials/MPC_PoolParty.MPC_PoolParty" "CausticsIntensity" _causticsintensity :!class /Script/Engine.KismetMaterialLibrary)
      (Rendering|Material|SetScalarParameterValue "/Game/Materials/MPC_PoolParty.MPC_PoolParty" "SunIntensity" _sunintensity :!class /Script/Engine.KismetMaterialLibrary)
      (Rendering|Components|Light|SetIntensity (Variables|/Script/Engine.Light|GetLightComponent _sunlight) (Math|Float|Lerp 0.0 1e+01 _sunintensity))
      (Rendering|Components|Light|SetLightColor (Variables|/Script/Engine.Light|GetLightComponent _sunlight) _skytint true)
      (Rendering|Material|SetVectorParameterValue "/Game/Materials/MPC_PoolParty.MPC_PoolParty" "NeonColour" _neontint :!class /Script/Engine.KismetMaterialLibrary))))

(event Collision|EventActorBeginOverlap
  (params (OtherActor :type Actor%20Object%20Reference)))

(event EventTick
  (params (DeltaSeconds :type Float%20%28single-precision%29)))

(fn ConstructionScript)